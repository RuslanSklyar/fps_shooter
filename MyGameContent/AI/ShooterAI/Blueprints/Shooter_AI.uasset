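; Shooter AI character that spawns a weapon at its gun socket and relays fire, reload and state-change events to the weapon and anim instance.
; AI state sets walk speed, and getters expose team, death status and patrol route.
; Damage events reduce health, with a large headshot multiplier.
; A looping timer polls health to trigger ragdoll death; its destroy and timer-pause steps are unwired, so polling never stops.
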(event Custom|EventDestroy
  (params (Delay :type Float%20%28single-precision%29) (Target :type Actor%20Object%20Reference))
  (Utilities|DestroyMacros 0.0))

(event Custom|Shoot
  (Variables|Default|SetAiming true)
  (Default|Fire (Variables|Default|GetWeapon) true))

(event Custom|ShootStop
  (Variables|Default|SetAiming false)
  (Default|Fire (Variables|Default|GetWeapon) false))

(event Custom|Reload
  (Default|Reload (Variables|Default|GetWeapon)))

(event Game|Damage|EventRadialDamage
  (params (DamageReceived :type Float%20%28single-precision%29) (DamageType :type Damage%20Type%20Object%20Reference) (Origin :type Vector :default "0, 0, 0") (HitInfo :type Hit%20Result%20Structure%20%28by%20ref%29) (InstigatedBy :type Controller%20Object%20Reference) (DamageCauser :type Actor%20Object%20Reference))
  (CallFunction|CalculetDamage "None" DamageReceived))

(event EventChangeState
  (params (NewState :type E_NPCState%20Enum :default "NewEnumerator0"))
  (Class|AIHelper|ChangeState(Message) (Components|SkeletalMesh|GetAnimInstance (Variables|Character|GetMesh)) NewState))

(event EventTakedamage
  (params (BoneName :type Name :default "None") (Damage :type Float%20%28single-precision%29) (Instigator :type Actor%20Object%20Reference))
  (CallFunction|CalculetDamage BoneName Damage Instigator))

(event EventModifyMovementSpeed
  (params (State :type E_NPCState%20Enum :default "NewEnumerator0"))
  (Variables|/Script/Engine.CharacterMovementComponent|SetMaxWalkSpeed (Variables|Character|GetCharacterMovement) (Utilities|Select :Index State :NewEnumerator0 1.8e+02 :NewEnumerator1 1.5e+02 :NewEnumerator2 4e+02 :NewEnumerator3 5e+02 :NewEnumerator4 0.0)))

(event EventBeginPlay
  (CallFunction|SetHealth)
  (CallFunction|SnapWeapon))

(fn ConstructionScript)

(fn SetHealth
  (Variables|Default|SetCurrentHealth (Variables|Default|GetMaxHeallth))
  (bind _returnvalue (Utilities|Time|SetTimerbyFunctionName 0 "Death" 0.1 true))
  (Variables|Default|SetTimer _returnvalue))

(fn Death
  (bind _mesh (Variables|Character|GetMesh))
  (if (<= (Variables|Default|GetCurrentHealth) 0.0)
    (Collision|SetActorEnableCollision false)
    (Class|SkeletalMeshComponent|SetAllBodiesSimulatePhysics _mesh true)
    (Collision|SetCollisionProfileName _mesh "Ragdoll" false :!class /Script/Engine.PrimitiveComponent)
    (Collision|SetCollisionEnabled (Variables|Collision|GetCapsuleComponent) "NoCollision")))

(fn CalculetDamage
  (params (A :type Name) (DamageLoc :type Float%20%28single-precision%29) (NewParam :type Actor%20Object%20Reference))
  (Development|PrintString "Damage" true true "(R=1.000000,G=0.000000,B=0.052273,A=1.000000)")
  (Variables|Default|SetDamageLoc DamageLoc)
  (if (Utilities|Name|Equal(Name) A "head")
    (Variables|Default|SetCurrentHealth (- (Variables|Default|GetCurrentHealth) (* (Variables|Default|GetDamageLoc) 1e+01)))
    (else
      (Variables|Default|SetCurrentHealth (- (Variables|Default|GetCurrentHealth) (Variables|Default|GetDamageLoc))))))

(fn SnapWeapon
  (bind _mesh (Variables|Character|GetMesh))
  (bind _returnvalue (Game|SpawnActorfromClass "/Game/MyGameContent/Weapon/BP_WeaponAI_Base.BP_WeaponAI_Base_C" (Transformation|GetSocketTransform _mesh "skt_gun1" "RTS_ParentBoneSpace") "Undefined" 0 0))
  (bind _output_get (Variables|Default|SetWeapon _returnvalue))
  (Transformation|AttachComponentToComponent _output_get (Variables|Character|GetMesh) (Class|SkinnedMeshComponent|GetSocketBoneName _mesh "skt_gun1") "KeepRelative" "KeepRelative" "KeepRelative" true))

(fn GetTeamId
  (return false))

(fn IsDead
  (return (<= (Variables|Default|GetCurrentHealth) 0.5)))

(fn PatrolRoute
  (return (Variables|Default|GetPatrol%20Route)))