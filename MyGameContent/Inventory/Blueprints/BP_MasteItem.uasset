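; BP_MasteItem is a base inventory item actor that can be picked up and declares hooks for weapon equipping and health use.
; Interact passes its class, Amount and ItemInfo to the inventory component's AddItem, then destroys the actor whether or not the add succeeds.
; BeginPlay caches the player character in CharRef.
; UseEqupmentWeapon and UseHealth are empty events here.
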(event Custom|UseEqupmentWeapon
  (params (Socket :type Name)))

(event Custom|UseHealth
  (params (IndexItem :type Integer)))

(event EventBeginPlay
  (bind _asbp_player_chatacter (Utilities|Casting|CastToBP_PlayerChatacter (Game|Player|GetPlayerPawn 0)))
  (Variables|Default|SetCharRef _asbp_player_chatacter))

(event EventInteract
  (params (InventoryComponent :type BPC%20Inventory%20Object%20Reference))
  (bind _success (Default|AddItem InventoryComponent (Utilities|GetClass self) (Variables|Default|GetAmount) (Variables|Default|GetItemInfo)))
  (if _success
    _
    (else
      _))
  (Actor|DestroyActor))

(fn ConstructionScript)