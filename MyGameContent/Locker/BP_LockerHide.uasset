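; Hideable locker that the player can interact with while inside its Box overlap, which enables input and opens a Gate.
; Interacting calls ToggleHide to flip the character's visibility and collision and blend the view between locker and character, while a timeline swings the door to 90 degrees.
; A short delay then re-enables input and reopens the Gate, which end overlap closes.
; CanUse blocks repeat use until the door timeline finishes.
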(event OnComponentBeginOverlap(Box)
  (params (OverlappedComponent :type Primitive%20Component%20Object%20Reference) (OtherActor :type Actor%20Object%20Reference) (OtherComp :type Primitive%20Component%20Object%20Reference) (OtherBodyIndex :type Integer) (bFromSweep :type Boolean) (SweepResult :type Hit%20Result%20Structure%20%28by%20ref%29))
  (bind _asbp_player_chatacter (Utilities|Casting|CastToBP_PlayerChatacter OtherActor))
  (Variables|Default|SetCharRef _asbp_player_chatacter)
  (Input|EnableInput (Game|GetPlayerController 0))
  (Utilities|FlowControl|Gate true) ; enters at Open
)

(event OnComponentEndOverlap(Box)
  (params (OverlappedComponent :type Primitive%20Component%20Object%20Reference) (OtherActor :type Actor%20Object%20Reference) (OtherComp :type Primitive%20Component%20Object%20Reference) (OtherBodyIndex :type Integer))
  (bind _returnvalue (Game|GetPlayerController 0))
  (Utilities|Casting|CastToBP_PlayerChatacter OtherActor)
  (Input|DisableInput _returnvalue)
  (Utilities|FlowControl|Gate true) ; enters at Close
)

(event Collision|EventActorBeginOverlap
  (params (OtherActor :type Actor%20Object%20Reference)))

(event EventTick
  (params (DeltaSeconds :type Float%20%28single-precision%29)))

(event EventInteract
  (params (InventoryComponent :type BPC%20Inventory%20Object%20Reference))
  (if (Variables|Default|GetCanUse)
    (Variables|Default|SetCanUse false)
    (Utilities|FlowControl|Gate true :!label _label
      (:Exit
        (Utilities|FlowControl|Sequence
          (:then_0
            (CallFunction|ToggleHide)
            (Utilities|FlowControl|Delay 0.2)
            (Input|EnableInput (Game|GetPlayerController 0))
            (goto _label Open))
          (:then_1
            (bind _newtrack_0 (Timeline|RotateDoor PlayFromStart)
              (:Update
                (Transformation|SetRelativeRotation (Variables|Default|GetDoor) (Math|Rotator|MakeRotator 0.0 0.0 (Math|Float|Lerp 0.0 9e+01 _newtrack_0)) false false))
              (:Finished
                (Variables|Default|SetCanUse true)))))))))

(fn ConstructionScript)

(fn ToggleHide
  (bind _charref (Variables|Default|GetCharRef))
  (bind _charref_2 (Variables|Default|GetCharRef))
  (if (Variables|Default|GetIsHide)
    (Variables|Default|SetIsHide false)
    (Rendering|SetActorHiddenInGame _charref false)
    (Collision|SetActorEnableCollision _charref true)
    (Game|Player|SetViewTargetwithBlend (Game|GetPlayerController 0) (Variables|Default|GetCharRef) 0.8 "VTBlend_Linear" 0.0 false)
    (else
      (Variables|Default|SetIsHide true)
      (Rendering|SetActorHiddenInGame _charref_2 true)
      (Collision|SetActorEnableCollision _charref_2 false)
      (Game|Player|SetViewTargetwithBlend (Game|GetPlayerController 0) self 0.8 "VTBlend_Linear" 0.0 false))))