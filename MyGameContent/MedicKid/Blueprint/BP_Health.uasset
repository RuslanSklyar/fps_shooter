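; BP_Health is a usable inventory item that heals the character.
; UseHealth acts only while health is below a hard-coded near-full threshold, adding the item's heal amount or just the missing health so it does not exceed the maximum.
; It then removes one unit from the given inventory slot and its weight through the inventory component.
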(event EventBeginPlay)

(event Collision|EventActorBeginOverlap
  (params (OtherActor :type Actor%20Object%20Reference)))

(event EventTick
  (params (DeltaSeconds :type Float%20%28single-precision%29)))

(event EventUseHealth
  (params (IndexItem :type Integer))
  (bind _inventorycomponent (Variables|Default|GetInventoryComponent))
  (bind _charref (Variables|Default|GetCharRef))
  (bind _healthmax (Variables|/Game/ThirdPersonBP/Blueprints/BP_PlayerChatacter.BP_PlayerChatacter_C|GetHealthMax _charref))
  (bind _health (Variables|/Game/ThirdPersonBP/Blueprints/BP_PlayerChatacter.BP_PlayerChatacter_C|GetHealth _charref))
  (if (< _health 99.5)
    (Default|AddHealth (Variables|Default|GetCharRef) (select (> _health (- _healthmax (Variables|Default|GetAddHealth))) (- _healthmax _health) (Variables|Default|GetAddHealth)))
    (Default|RemoveItematIndex _inventorycomponent IndexItem 1)
    (Default|RemoveWeightfromItem _inventorycomponent (Utilities|GetClass self) 1)))

(fn ConstructionScript
  (|CallParentFunction))