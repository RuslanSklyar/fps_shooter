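; AWP sniper rifle weapon Blueprint that adds stepped scope zoom.
; ZoomIn and ZoomOut, gated by CanScope, step the SceneCaptureComponent2D field of view within a clamped range.
; Each step also nudges the capture component's world pitch, up on zoom in and down on zoom out.
; BeginPlay and construction only call the parent; Tick is empty, and similar Camera pitch adjustments are left unconnected.
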(event Custom|ZoomIn
  (bind _scenecapturecomponent2d (Variables|Default|GetSceneCaptureComponent2D))
  (bind _returnvalue (Transformation|GetWorldRotation _scenecapturecomponent2d))
  ;[1 1 1] Зум для авп
  (if (and (Variables|Default|GetCan%20Scope) (> (Variables|/Script/Engine.SceneCaptureComponent2D|GetFOVAngle _scenecapturecomponent2d) 1.0))
    (Variables|/Script/Engine.SceneCaptureComponent2D|SetFOVAngle _scenecapturecomponent2d (Math|Float|Clamp(Float) (- (Variables|/Script/Engine.SceneCaptureComponent2D|GetFOVAngle _scenecapturecomponent2d) 1.0) 1.0 1e+01))
    (Transformation|SetWorldRotation _scenecapturecomponent2d (Math|Rotator|MakeRotator (.roll _returnvalue) (+ (.pitch _returnvalue) 0.5) (.yaw _returnvalue)) false false)))

(event Custom|ZoomOut
  (bind _scenecapturecomponent2d (Variables|Default|GetSceneCaptureComponent2D))
  (bind _returnvalue (Transformation|GetWorldRotation _scenecapturecomponent2d))
  ;[1 1 1] Зум для авп
  (if (and (Variables|Default|GetCan%20Scope) (< (Variables|/Script/Engine.SceneCaptureComponent2D|GetFOVAngle _scenecapturecomponent2d) 1e+01))
    (Variables|/Script/Engine.SceneCaptureComponent2D|SetFOVAngle _scenecapturecomponent2d (Math|Float|Clamp(Float) (+ (Variables|/Script/Engine.SceneCaptureComponent2D|GetFOVAngle _scenecapturecomponent2d) 1.0) 1.0 1e+01))
    (Transformation|SetWorldRotation _scenecapturecomponent2d (Math|Rotator|MakeRotator (.roll _returnvalue) (- (.pitch _returnvalue) 0.5) (.yaw _returnvalue)) false false)))

(event EventBeginPlay
  (|CallParentFunction))

(event Collision|EventActorBeginOverlap
  (params (OtherActor :type Actor%20Object%20Reference))
  (|CallParentFunction OtherActor) ; This node is disabled and will not be called.\nDrag off pins to build functionality.
)

(event EventTick
  (params (DeltaSeconds :type Float%20%28single-precision%29)))

(fn ConstructionScript
  (|CallParentFunction))