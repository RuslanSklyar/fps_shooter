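; BP_Bullet is a projectile actor that delivers damage on impact.
; On hit, damageable characters receive damage and bone name via the TakeDamage interface, with floating text showing damage or "HeadShot" for head hits.
; Non-damageable hits leave a normal-aligned decal; both completed paths destroy the bullet.
; Tick sphere-traces ahead and casts hits to Shooter_AI, but does nothing with the result.
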(event EventTick
  (params (DeltaSeconds :type Float%20%28single-precision%29))
  (bind _returnvalue (Transformation|GetActorLocation))
  (bind (_outhit _returnvalue_2) (Collision|SphereTraceByChannel _returnvalue (+ _returnvalue (* (Math|Vector|GetForwardVector (Transformation|GetWorldRotation (Variables|Default|GetSphere))) 5e+02)) 5e+01 "TraceTypeQuery1" false (Utilities|Array|MakeArray self) "None"))
  (if _returnvalue_2
    (Utilities|Casting|CastToShooter_AI (.HitActor (Collision|BreakHitResult _outhit)))))

(event Collision|EventHit
  (params (MyComp :type Primitive%20Component%20Object%20Reference) (Other :type Actor%20Object%20Reference) (OtherComp :type Primitive%20Component%20Object%20Reference) (bSelfMoved :type Boolean) (HitLocation :type Vector :default "0, 0, 0") (HitNormal :type Vector :default "0, 0, 0") (NormalImpulse :type Vector :default "0, 0, 0") (Hit :type Hit%20Result%20Structure%20%28by%20ref%29))
  (bind (_bblockinghit _binitialoverlap _time _distance _location _impactpoint _normal _impactnormal _physmat _hitactor _hitcomponent _hitbonename) (Collision|BreakHitResult Hit))
  (if (Utilities|DoesObjectImplementInterface Other "/Game/ThirdPersonBP/Blueprints/BPI_DrawDamageInScreen/TakeDamage.TakeDamage_C")
    (bind _ascharacter (Utilities|Casting|CastToCharacter Other))
    (Class|TakeDamage|Takedamage(Message) Other _hitbonename (Variables|Default|GetDamage) (Game|GetInstigator _ascharacter))
    (Game|SpawnActorfromClass "/Game/ThirdPersonBP/Blueprints/BPI_DrawDamageInScreen/BP_FloatingText.BP_FloatingText_C" (Math|Transform|MakeTransform HitLocation "0, 0, 0" "1,1,1") "Undefined" 0 (select (Utilities|Name|Equal(Name) _hitbonename "head") "HeadShot" (Utilities|Text|ToText(Float) (Variables|Default|GetDamage) "HalfToEven" false true 1 324 0 0)) 0)
    (else
      (Game|SpawnActorfromClass "/Game/MyGameContent/Weapon/Decal/Bullet/Blueprints/BP_Decal.BP_Decal_C" (Math|Transform|MakeTransform _location (Math|Conversions|RotationFromXVector _normal) "0.030000,0.030000,0.030000") "Undefined" 0 0)))
  (Actor|DestroyActor))

(fn ConstructionScript)