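; Base weapon Blueprint providing shooting, reloading, fire-mode switching and a toggleable flashlight, with stats loaded from DT_Weapom at construction.
; FirePress loops through RetriggerableDelay for single, burst and auto fire, playing montages, muzzle flash and recoil.
; Each shot spawns BP_Bullet actors at the camera trace's hit location, with random spread and damage.
; Reloading deducts inventory ammo after a delay, while Tick traces from the muzzle to position the laser endpoint.
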(event Custom|Lights
  (bind _spotlight (Variables|Components|GetSpotLight))
  ;[1 1 1] Фонарик
  (Utilities|FlowControl|FlipFlop
    (:A
      (Variables|Default|SetIsFlash false)
      (Rendering|SetVisibility _spotlight false false))
    (:B
      (Variables|Default|SetIsFlash true)
      (Rendering|SetVisibility _spotlight true false))))

(event Custom|ZoomIn
  ;[1 1 1] Каст на персонажа
)

(event Custom|ZoomOut
  ;[1 1 1] Каст на персонажа
)

(event Custom|ReloadWeapon
  ;[1 1 1] Перезаписываем патроны в WeaponData
  (if (Variables|Default|GetIsReload)
    (if (> (Variables|Default|GetAmmo%20Max) 0)
      (Variables|Default|SetNeedAmmo (- (Variables|Default|GetAmmo%20in%20Clip) (Variables|Default|GetAmmo%20Current)))
      (if (> (Variables|Default|GetNeedAmmo) (Variables|Default|GetAmmo%20Max))
        (bind _output_get (Variables|Default|SetAmmo%20Current (+ (Variables|Default|GetAmmo%20Max) (Variables|Default|GetAmmo%20Current))))
        (CallFunction|DestroyAmmoinInventory _output_get)
        (Variables|Default|SetIsReload false)
        (Variables|Default|SetAmmo%20Max 0)
        (Default|RemoveWeightfromItem (Variables|Default|GetInventoryComponent) (Variables|Default|GetAmmoClass) _output_get)
        (else
          (Variables|Default|SetAmmo%20Current (+ (Variables|Default|GetAmmo%20Current) (Variables|Default|GetNeedAmmo)))
          (CallFunction|DestroyAmmoinInventory (Variables|Default|GetNeedAmmo))
          (Variables|Default|SetIsReload false)
          (Variables|Default|SetAmmo%20Max (- (Variables|Default|GetAmmo%20Max) (Variables|Default|GetNeedAmmo)))
          (Default|RemoveWeightfromItem (Variables|Default|GetInventoryComponent) (Variables|Default|GetAmmoClass) (Variables|Default|GetNeedAmmo)))))))

(event Custom|FirePress
  (params (TrigerBullet :type Boolean))
  ;[1 1 1] Реализация выстрела
  (bind _output_get (Variables|Default|SetFiring TrigerBullet))
  (if (Math|Boolean|ANDBoolean (CallFunction|HasAmmo) (CallFunction|CanShoot) _output_get) :!label _label
    (switch Utilities|FlowControl|Switch|SwitchonEnum_FireMode (Variables|Default|GetFire%20Mode)
      (:NewEnumerator0
        (Variables|Default|SetFireRateDelay true)
        (CallFunction|SpawnProjectail)
        (Utilities|LightsBullet)
        (Utilities|FlowControl|RetriggerableDelay (Variables|Default|GetFire%20Rate))
        (Variables|Default|SetFireRateDelay false)
        (Variables|Default|SetFiring false))
      (:NewEnumerator1
        (if (> (.BulletsInBurst (Utilities|Struct|BreakStruct_WeaponData (Variables|Default|GetWeaponData))) (Variables|Default|GetCurrentBulletsInBurst))
          (Variables|Default|SetFireRateDelay true)
          (Math|Integer|IncrementInt (Variables|Default|GetCurrentBulletsInBurst)
            (:%20%20
              (CallFunction|SpawnProjectail)
              (Utilities|LightsBullet)
              (Utilities|FlowControl|RetriggerableDelay (Variables|Default|GetFire%20Rate))
              (Variables|Default|SetFireRateDelay false)
              (goto _label)))
          (else
            (Variables|Default|SetCurrentBulletsInBurst 0)
            (Variables|Default|SetFiring false))))
      (:NewEnumerator2
        (Variables|Default|SetFireRateDelay true)
        (CallFunction|SpawnProjectail)
        (Utilities|LightsBullet)
        (Utilities|FlowControl|RetriggerableDelay (Variables|Default|GetFire%20Rate))
        (Variables|Default|SetFireRateDelay false)
        (goto _label)))
    (elif (not (CallFunction|HasAmmo))
      (if (CallFunction|CanShoot)
        (CallFunction|SoundNoAmmo (.NoAmmoSound (Utilities|Struct|BreakStruct_WeaponData (Variables|Default|GetWeaponData))))
        (else
          (CallFunction|Reloading))))))

(event Custom|Reloading
  ;[1 1 1] Перезарядка
  (if (not (== (Variables|Default|GetAmmo%20Max) 0))
    (if (not (== (Variables|Default|GetAmmo%20in%20Clip) (Variables|Default|GetAmmo%20Current)))
      (if (not (Variables|Default|GetIsReload))
        (Variables|Default|SetIsReload true)
        (CallFunction|PlayMontage (.ReloadMontage (Utilities|Struct|BreakStruct_WeaponData (Variables|Default|GetWeaponData))) "/Game/Mannequin/Animations/Montage/Reload_Rifle_Hip_Montage.Reload_Rifle_Hip_Montage")
        (Utilities|FlowControl|Delay (Variables|Default|GetReload%20Delay))
        (CallFunction|ReloadWeapon)))))

(event Custom|FireMode
  (bind _weapondata (Variables|Default|GetWeaponData))
  (bind (_ammomax _ammocurrent _bursttype _canscope) (Utilities|Struct|BreakStruct_WeaponData _weapondata))
  ;[1 1 1] Переключение режима стрельбы
  (if _canscope
    (Variables|Default|SetFire%20Mode "NewEnumerator0")
    (elif _bursttype
      (switch Utilities|FlowControl|Switch|SwitchonEnum_FireMode (Variables|Default|GetFire%20Mode)
        (:NewEnumerator0
          (Variables|Default|SetFire%20Mode "NewEnumerator1"))
        (:NewEnumerator1
          (Variables|Default|SetFire%20Mode "NewEnumerator2" :!label _label))
        (:NewEnumerator2
          (Variables|Default|SetFire%20Mode "NewEnumerator0" :!label _label_2)))
      (else
        (switch Utilities|FlowControl|Switch|SwitchonEnum_FireMode (Variables|Default|GetFire%20Mode)
          (:NewEnumerator0
            (goto _label))
          (:NewEnumerator2
            (goto _label_2)))))))

(event Collision|EventActorBeginOverlap
  (params (OtherActor :type Actor%20Object%20Reference)))

(event EventTick
  (params (DeltaSeconds :type Float%20%28single-precision%29))
  (bind _weaponmesh (Variables|Components|GetWeaponMesh))
  (bind _returnvalue (Transformation|GetSocketLocation _weaponmesh "Muzzle"))
  (bind (_outhit _returnvalue_2) (Collision|LineTraceByChannel _returnvalue (+ _returnvalue (* (Math|Vector|GetForwardVector _weaponmesh) 56465464.0)) "TraceTypeQuery1" false 0 "ForOneFrame"))
  (if _returnvalue_2
    (Transformation|SetWorldLocation (Variables|Default|GetLazerEndPoint) (.Location (Collision|BreakHitResult _outhit)) false false)))

(event EventUseEqupmentWeapon
  (params (Socket :type Name :default "None")))

(fn ConstructionScript
  (bind _returnvalue (Utilities|GetDataTableRow "/Game/MyGameContent/Weapon/List/DT_Weapom.DT_Weapom" (Variables|Default|GetWeaponRowName))
    (:then
      (bind _output_get (Variables|Default|SetWeaponData _returnvalue))
      (Variables|Default|SetFire%20Mode (.FireMode (Utilities|Struct|BreakStruct_WeaponData _output_get)))
      (Variables|Default|SetMazzle%20Name (.MazzleName (Utilities|Struct|BreakStruct_WeaponData _output_get)))
      (Variables|Default|SetFire%20Rate (.FireRate (Utilities|Struct|BreakStruct_WeaponData _output_get)))
      (Variables|Default|SetReload%20Delay (.ReloadDelay (Utilities|Struct|BreakStruct_WeaponData _output_get)))
      (Variables|Default|SetWeapon%20Spray (.WeaponSpray (Utilities|Struct|BreakStruct_WeaponData _output_get)))
      (Variables|Default|SetAmmo%20Max (.AmmoMax (Utilities|Struct|BreakStruct_WeaponData _output_get)))
      (Variables|Default|SetAmmo%20in%20Clip (.AmmoInClip (Utilities|Struct|BreakStruct_WeaponData _output_get)))
      (Variables|Default|SetAmmo%20Current (.AmmoCurrent (Utilities|Struct|BreakStruct_WeaponData _output_get)))
      (Variables|Default|SetBullets%20in%20Shot (.BulletsInShot (Utilities|Struct|BreakStruct_WeaponData _output_get)))
      (Variables|Default|SetCan%20Scope (.CanScope (Utilities|Struct|BreakStruct_WeaponData _output_get)))
      (Variables|Default|SetPLState (.PLState (Utilities|Struct|BreakStruct_WeaponData _output_get))))))

(fn PlayMontage
  (params (WeaponAnim :type Anim%20Montage%20Object%20Reference) (CharAnim :type Anim%20Montage%20Object%20Reference))
  (Animation|Montage|MontagePlay (Components|SkeletalMesh|GetAnimInstance (Variables|Components|GetWeaponMesh)) WeaponAnim 1.0 "MontageLength" 0.0 false)
  (Animation|Montage|MontagePlay (Components|SkeletalMesh|GetAnimInstance (Variables|/Script/Engine.Character|GetMesh (Variables|Default|GetCharRef))) CharAnim 1.0 "Duration" 0.0 false))

(fn SpawnProjectail
  (bind _weapondata (Variables|Default|GetWeaponData))
  (bind (_mindamage _maxdamage _ammomax _ammocurrent _weaponrecoil) (Utilities|Struct|BreakStruct_WeaponData _weapondata))
  (CallFunction|PlayMontage (.FiringMontage (Utilities|Struct|BreakStruct_WeaponData (Variables|Default|GetWeaponData))) (select (Variables|/Game/ThirdPersonBP/Blueprints/BP_PlayerChatacter.BP_PlayerChatacter_C|GetAiming (Variables|Default|GetCharRef)) "/Game/Mannequin/Animations/Montage/Fire_Rifle_Ironsights_Montage.Fire_Rifle_Ironsights_Montage" "/Game/Mannequin/Animations/Montage/Fire_Rifle_Hip_Montage.Fire_Rifle_Hip_Montage"))
  (for _index (range 0 (Variables|Default|GetBullets%20in%20Shot))
    (bind (_newparam _newparam1) (CallFunction|CalculetDirection))
    (bind _transform (CallFunction|CalculetFinalDirection _newparam _newparam1))
    (Game|SpawnActorfromClass "/Game/MyGameContent/Weapon/BP_Bullet.BP_Bullet_C" _transform "Undefined" 0 (Math|Random|RandomFloatinRange _mindamage _maxdamage) 0)
    (Default|WeaponRecoil (Variables|Default|GetCharRef) _weaponrecoil))
  (Math|Integer|DecrementInt (Variables|Default|GetAmmo%20Current)))

(fn CanShoot
  (return (Math|Boolean|ANDBoolean (Variables|Default|GetFiring) (not (Variables|Default|GetFireRateDelay)) (not (Variables|Default|GetIsReload)))))

(fn SoundNoAmmo
  (params (Sound :type Sound%20Base%20Object%20Reference))
  (Audio|PlaySoundatLocation Sound (Transformation|GetWorldLocation (Variables|Components|GetWeaponMesh)) "0, 0, 0" 1.0 1.0 0.0 0 0 0))

(fn HasAmmo
  (return (> (Variables|Default|GetAmmo%20Current) 0)))

(fn CalculetDirection
  (bind _camera (Variables|Components|GetCamera))
  (bind _charref (Variables|Default|GetCharRef))
  (bind _returnvalue (Transformation|GetWorldLocation _camera))
  (bind _returnvalue_2 (Math|Vector|GetForwardVector _camera))
  (bind _camera_2 (Variables|/Game/ThirdPersonBP/Blueprints/BP_PlayerChatacter.BP_PlayerChatacter_C|GetCamera _charref))
  (bind _tcamera (Variables|/Game/ThirdPersonBP/Blueprints/BP_PlayerChatacter.BP_PlayerChatacter_C|GettCamera _charref))
  (bind _fcamera (Variables|/Game/ThirdPersonBP/Blueprints/BP_PlayerChatacter.BP_PlayerChatacter_C|GetfCamera _charref))
  (bind _aiming (Variables|/Game/ThirdPersonBP/Blueprints/BP_PlayerChatacter.BP_PlayerChatacter_C|GetAiming _charref))
  (bind _returnvalue_3 (select _camera_2 _tcamera _fcamera))
  (bind _returnvalue_4 (Transformation|GetWorldLocation _returnvalue_3))
  (bind _returnvalue_5 (Math|Vector|GetForwardVector _returnvalue_3))
  (bind _returnvalue_6 (select _aiming _returnvalue _returnvalue_4))
  (bind _returnvalue_7 (select _aiming _returnvalue_2 _returnvalue_5))
  (bind _returnvalue_8 (* _returnvalue_7 95956533248.0))
  (bind (_outhit _returnvalue_9) (Collision|LineTraceByChannel _returnvalue_6 (+ _returnvalue_8 _returnvalue_6) "TraceTypeQuery1" false (Utilities|Array|MakeArray (Variables|Default|GetCharRef)) "ForDuration" true "(R=1.000000,G=0.000000,B=0.000000,A=1.000000)" "(R=0.000000,G=1.000000,B=0.000000,A=1.000000)" 1e+01))
  (return (.Location (Collision|BreakHitResult _outhit)) (Math|Rotator|FindLookatRotation (.Location (Collision|BreakHitResult _outhit)) (Math|Vector|SelectVector (.Location (Collision|BreakHitResult _outhit)) _returnvalue_8 _returnvalue_9))))

(fn CalculetFinalDirection
  (params (Location :type Vector) (Rotation :type Rotator))
  (bind _weapon_spray (Variables|Default|GetWeapon%20Spray))
  (bind _weapon_spray_2 (Variables|Default|GetWeapon%20Spray))
  (bind _returnvalue (* _weapon_spray_2 -1.0))
  (return (Math|Transform|MakeTransform Location (Math|Rotator|CombineRotators Rotation (Math|Rotator|MakeRotator (Math|Random|RandomFloatinRange _returnvalue _weapon_spray) (Math|Random|RandomFloatinRange _returnvalue _weapon_spray) (Math|Random|RandomFloatinRange _returnvalue _weapon_spray))))))

(fn CheckAmmoinSlots
  (bind (_array_element _array_index) (Utilities|Array|ForEachLoopwithBreak (Variables|/Game/MyGameContent/Inventory/Blueprints/BPC_Inventory.BPC_Inventory_C|GetSlots (Variables|Default|GetInventoryComponent)) :!label _label)
    (:LoopBody
      (if (== (.ItemActor (Utilities|Struct|BreakS_InventarySlot _array_element)) (Variables|Default|GetAmmoClass))
        (LocalVariables|SetLocalIndex _array_index)
        (goto _label Break)))
    (:Completed
      (return (LocalVariables|GetLocalIndex)))))

(fn DestroyAmmoinInventory
  (params (Amount :type Integer))
  (Default|RemoveItematIndex (Variables|Default|GetInventoryComponent) (CallFunction|CheckAmmoinSlots) Amount))

(fn IsLazer
  (Utilities|FlowControl|Sequence
    (:then_0
      (Variables|Default|GetIsLaser
        (:then)
        (:else
          (bind _returnvalue (Game|SpawnActorfromClass "/Game/MyGameContent/LazerParticleVisiual.LazerParticleVisiual_C" (Math|Transform|MakeTransform "0, 0, 0" "0, 0, 0" "1,1,1") "AlwaysSpawn" self (Game|GetInstigator)))
          (Variables|Default|SetIsLaser _returnvalue))))
    (:then_1
      (Variables|Default|GetIsLaser
        (:then
          (Variables|/Game/MyGameContent/LazerParticleVisiual.LazerParticleVisiual_C|SetStartLocation (Variables|Default|GetIsLaser) (Transformation|GetWorldLocation (Variables|Default|GetLazerStartPoint)))
          (Variables|/Game/MyGameContent/LazerParticleVisiual.LazerParticleVisiual_C|SetEndLocation (Variables|Default|GetIsLaser) (Transformation|GetWorldLocation (Variables|Default|GetLazerEndPoint))))
        (:else)))))