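; Explosive barrel that loses health when hit by BP_Bullet, which it destroys.
; At low health it ignites with particles and a timeline-driven light, exploding after a delay, or at once when health is depleted.
; The blast expands DamageSphere to trigger overlaps, fires a radial impulse, plays sound and destroys the barrel.
; Overlapped TakeDamage actors react: players take damage and camera shake, while other barrels have health reset to ignite in a chain.
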(event OnComponentBeginOverlap(DamageSphere)
  (params (OverlappedComponent :type Primitive%20Component%20Object%20Reference) (OtherActor :type Actor%20Object%20Reference) (OtherComp :type Primitive%20Component%20Object%20Reference) (OtherBodyIndex :type Integer) (bFromSweep :type Boolean) (SweepResult :type Hit%20Result%20Structure%20%28by%20ref%29))
  (if (Utilities|DoesObjectImplementInterface OtherActor "/Game/ThirdPersonBP/Blueprints/BPI_DrawDamageInScreen/TakeDamage.TakeDamage_C")
    (Utilities|FlowControl|Sequence
      (:then_0
        (bind _asbp_player_chatacter (Utilities|Casting|CastToBP_PlayerChatacter OtherActor))
        (Default|Takedamage _asbp_player_chatacter "None" 7e+01)
        (Variables|/Game/ThirdPersonBP/Blueprints/BP_PlayerChatacter.BP_PlayerChatacter_C|SetCamShakeCamera _asbp_player_chatacter true))
      (:then_1
        (bind _asbp_barl (Utilities|Casting|CastToBP_Barl OtherActor))
        (Variables|BP_Barl_C|SetHealthBarl _asbp_barl 7e+01)
        (CallFunction|BarlEvent _asbp_barl)))))

(event Custom|BarlEvent
  (Variables|Default|SetHealthBarl (- (Variables|Default|GetHealthBarl) 25.0))
  (if (and (<= (Variables|Default|GetHealthBarl) 55.0) (> (Variables|Default|GetHealthBarl) 0.0))
    (Components|Activation|Activate (Variables|Default|GetParticleSystem) false)
    (Rendering|SetVisibility (Variables|Default|GetPointLight) true false)
    (bind _newtrack_0 (Timeline|Timeline_0 Play)
      (:Update
        (Rendering|Components|Light|SetIntensity (Variables|Default|GetPointLight) _newtrack_0)
        (Utilities|FlowControl|Delay 3.0)
        (Utilities|IsValid self
          (:Is%20Valid
            (Components|Sphere|SetSphereRadius (Variables|Default|GetDamageSphere) 8e+02 true :!label _label)
            (Class|RadialForceComponent|FireImpulse (Variables|Default|GetRadialForce))
            (Audio|PlaySoundatLocation "/Game/StarterContent/Audio/Explosion01.Explosion01" (Transformation|GetActorLocation self) "0, 0, 0" 1.0 1.0 0.0 0 0 0)
            (Actor|DestroyActor)))))
    (elif (<= (Variables|Default|GetHealthBarl) 5.0)
      (Utilities|IsValid self
        (:Is%20Valid
          (goto _label))))))

(event Collision|EventHit
  (params (MyComp :type Primitive%20Component%20Object%20Reference) (Other :type Actor%20Object%20Reference) (OtherComp :type Primitive%20Component%20Object%20Reference) (bSelfMoved :type Boolean) (HitLocation :type Vector :default "0, 0, 0") (HitNormal :type Vector :default "0, 0, 0") (NormalImpulse :type Vector :default "0, 0, 0") (Hit :type Hit%20Result%20Structure%20%28by%20ref%29))
  (bind _asbp_bullet (Utilities|Casting|CastToBP_Bullet Other))
  (Actor|DestroyActor _asbp_bullet)
  (CallFunction|BarlEvent))

(fn ConstructionScript)