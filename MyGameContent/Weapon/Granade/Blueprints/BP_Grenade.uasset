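; Grenade actor that explodes on a timed fuse from BeginPlay and switches on physics simulation when it hits something.
; On detonation it enables and enlarges the damage sphere, fires a radial impulse, plays sound and particles, then destroys itself shortly after.
; Damage uses overlap events from that sphere, messaging actors through the TakeDamage interface.
; Overlapped BP_Barl actors also get their health set directly and their BarlEvent triggered.
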(event OnComponentBeginOverlap(SphereDamage)
  (params (OverlappedComponent :type Primitive%20Component%20Object%20Reference) (OtherActor :type Actor%20Object%20Reference) (OtherComp :type Primitive%20Component%20Object%20Reference) (OtherBodyIndex :type Integer) (bFromSweep :type Boolean) (SweepResult :type Hit%20Result%20Structure%20%28by%20ref%29))
  (Utilities|FlowControl|Sequence
    (:then_0
      (if (Utilities|DoesObjectImplementInterface OtherActor "/Game/ThirdPersonBP/Blueprints/BPI_DrawDamageInScreen/TakeDamage.TakeDamage_C")
        (Class|TakeDamage|Takedamage(Message) OtherActor "None" (Variables|Default|GetDamage))))
    (:then_1
      (bind _asbp_barl (Utilities|Casting|CastToBP_Barl OtherActor))
      (Variables|/Game/MyGameContent/Weapon/Barl/Blueprints/BP_Barl.BP_Barl_C|SetHealthBarl _asbp_barl 3e+01)
      (Default|BarlEvent _asbp_barl))))

(event EventBeginPlay
  (Utilities|FlowControl|Delay 2.0)
  (Collision|SetCollisionEnabled (Variables|Default|GetSphereDamage) "QueryOnly")
  (Components|Sphere|SetSphereRadius (Variables|Default|GetSphereDamage) 5e+02 true)
  (Class|RadialForceComponent|FireImpulse (Variables|Default|GetRadialForce))
  (Audio|PlaySoundatLocation "/Game/StarterContent/Audio/Explosion01.Explosion01" (Transformation|GetActorLocation) "0, 0, 0" 1.0 1.0 0.0 0 0 0)
  (Components|Activation|Activate (Variables|Default|GetParticleSystem) false)
  (Utilities|FlowControl|Delay 0.1)
  (Actor|DestroyActor))

(event Collision|EventHit
  (params (MyComp :type Primitive%20Component%20Object%20Reference) (Other :type Actor%20Object%20Reference) (OtherComp :type Primitive%20Component%20Object%20Reference) (bSelfMoved :type Boolean) (HitLocation :type Vector :default "0, 0, 0") (HitNormal :type Vector :default "0, 0, 0") (NormalImpulse :type Vector :default "0, 0, 0") (Hit :type Hit%20Result%20Structure%20%28by%20ref%29))
  (Physics|SetSimulatePhysics (Variables|Default|GetSphere) true))

(fn ConstructionScript)