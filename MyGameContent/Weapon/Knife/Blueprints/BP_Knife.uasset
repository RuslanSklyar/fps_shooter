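; Knife weapon Blueprint that damages actors touched by its capsule and plays an attack montage on the owning character.
; Capsule overlap sends a fixed damage message through the TakeDamage interface, excluding the owner, with no check on the firing state.
; FirePress plays Sprint_Fwd_Rifle_Montage and clears the Firing flag after a retriggerable delay of the montage's length.
; Lights and both reload events are empty stubs.
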(event OnComponentBeginOverlap(CapsuleDamageCollision)
  (params (OverlappedComponent :type Primitive%20Component%20Object%20Reference) (OtherActor :type Actor%20Object%20Reference) (OtherComp :type Primitive%20Component%20Object%20Reference) (OtherBodyIndex :type Integer) (bFromSweep :type Boolean) (SweepResult :type Hit%20Result%20Structure%20%28by%20ref%29))
  (if (and (Utilities|DoesObjectImplementInterface OtherActor "/Game/ThirdPersonBP/Blueprints/BPI_DrawDamageInScreen/TakeDamage.TakeDamage_C") (!= OtherActor (Variables|Default|GetCharRef)))
    (Class|TakeDamage|Takedamage(Message) OtherActor "None" 45.0)))

(event EventBeginPlay
  (|CallParentFunction) ; This node is disabled and will not be called.\nDrag off pins to build functionality.
)

(event Collision|EventActorBeginOverlap
  (params (OtherActor :type Actor%20Object%20Reference))
  (|CallParentFunction OtherActor) ; This node is disabled and will not be called.\nDrag off pins to build functionality.
)

(event EventTick
  (params (DeltaSeconds :type Float%20%28single-precision%29))
  (|CallParentFunction DeltaSeconds) ; This node is disabled and will not be called.\nDrag off pins to build functionality.
)

(event EventFirePress
  (params (TrigerBullet :type Boolean))
  (bind _output_get (Variables|Default|SetFiring TrigerBullet))
  (if _output_get
    (bind _returnvalue (Animation|PlayAnimMontage (Variables|Default|GetCharRef) "/Game/Sprint_Fwd_Rifle_Montage.Sprint_Fwd_Rifle_Montage" 1.0 "None"))
    (Utilities|FlowControl|RetriggerableDelay _returnvalue)
    (Variables|Default|SetFiring false)))

(event EventLights)

(event EventReloadWeapon)

(event EventReloading)

(fn ConstructionScript)